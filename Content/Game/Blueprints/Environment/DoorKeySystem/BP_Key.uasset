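; BP_Key is an interactable key pickup for the door key system, tinted green, red or blue by its index.
; BeginPlay caches the first-person game mode, and Interact overwrites that mode's Keys value with this key's index, prints an acquired message with its name, then destroys the actor.
; The construction script selects the key material from the index; an unconnected array and card-visibility pickup path remains unused.
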(event EventBeginPlay
  (bind _asbp_first_person_game_mode (Utilities|Casting|CastToBP_FirstPersonGameMode (Game|GetGameMode)))
  (Variables|Default|SetAs%20BP%20First%20Person%20Game%20Mode _asbp_first_person_game_mode))

(event EventInteract
  (params (CharRef :type BP%20Player%20Object%20Reference))
  (bind _output_get (Variables|/Game/Game/Blueprints/Player/BP_FirstPersonGameMode.BP_FirstPersonGameMode_C|SetKeys (Variables|Default|GetAs%20BP%20First%20Person%20Game%20Mode) (Variables|Default|GetkeyIndex)))
  (Development|PrintString (Utilities|String|Append "Key" (Utilities|Array|Get(acopy) (Variables|Default|GetNames) _output_get) "Acquired"))
  (Actor|DestroyActor))

(fn ConstructionScript
  (Rendering|Material|SetMaterial (Variables|Default|GetKey) 0 (Utilities|Select :Index (Variables|Default|GetkeyIndex) :Option%200 "/Game/Game/Materials/M_Green.M_Green" :Option%201 "/Game/Game/Materials/M_Red.M_Red" :Option%202 "/Game/Game/Materials/M_Blue.M_Blue")))