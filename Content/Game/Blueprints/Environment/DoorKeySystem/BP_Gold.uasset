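; Gold pickup that adds a random amount to the player's gold in BP_FirstPersonGameMode when interacted with, then destroys itself.
; The construction script rolls the amount (GoldIndex) and uses a macro to scatter randomly offset and scaled mesh components.
; The macro's checks all test GoldIndex >= 0, so they always pass and the pile size does not follow the value.
; BeginPlay caches the game mode and shows the amount on a text render.
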(event EventBeginPlay
  (bind _asbp_first_person_game_mode (Utilities|Casting|CastToBP_FirstPersonGameMode (Game|GetGameMode)))
  (Variables|Default|SetAs%20BP%20First%20Person%20Game%20Mode _asbp_first_person_game_mode)
  (Rendering|Components|TextRender|SetText (Variables|Default|GetTextRender) (|GenerictoText (Variables|Default|GetGoldIndex))))

(event EventInteract
  (bind _output_get (Variables|/Game/Game/Blueprints/Player/BP_FirstPersonGameMode.BP_FirstPersonGameMode_C|SetPlayerGold (Variables|Default|GetAs%20BP%20First%20Person%20Game%20Mode) (+ (Variables|/Game/Game/Blueprints/Player/BP_FirstPersonGameMode.BP_FirstPersonGameMode_C|GetPlayerGold (Variables|Default|GetAs%20BP%20First%20Person%20Game%20Mode)) (Variables|Default|GetGoldIndex))))
  (Development|PrintString (Utilities|String|Append "Current Gold" (Utilities|String|ToString(Integer) _output_get)))
  (Actor|DestroyActor))

(fn ConstructionScript
  (Variables|Default|SetGoldIndex (Math|Random|RandomIntegerinRange 1 99))
  (Utilities|AddStaticMesh (>= (Variables|Default|GetGoldIndex) 0)
    (:Out
      _)
    (:False
      _))
  (Utilities|AddStaticMesh (>= (Variables|Default|GetGoldIndex) 0)
    (:Out
      _)
    (:False
      _))
  (Utilities|AddStaticMesh (>= (Variables|Default|GetGoldIndex) 0)))