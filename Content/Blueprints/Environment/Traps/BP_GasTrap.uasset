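; BP_GasTrap is a gas trap that deals repeated damage to the player while they stand inside its damage collider.
; Overlap begin starts a looping timer that calls DamageUpdate on the player cached at BeginPlay, and overlap end clears it.
; A player-bound DP trap event with a matching TrapType disables the collider and destroys the gas component.
; The grid-based gas scaling in the construction script is disconnected.
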(event OnComponentBeginOverlap(DamageColl)
  (params (OverlappedComponent :type Primitive%20Component%20Object%20Reference) (OtherActor :type Actor%20Object%20Reference) (OtherComp :type Primitive%20Component%20Object%20Reference) (OtherBodyIndex :type Integer) (bFromSweep :type Boolean) (SweepResult :type Hit%20Result%20Structure%20%28by%20ref%29))
  (if (== OtherActor (Variables|Default|GetAs%20BP%20First%20Person%20Character))
    (Utilities|Time|SetTimerbyFunctionName 0 "DOT" (Variables|Default|GetGas_Time) true)))

(event OnComponentEndOverlap(DamageColl)
  (params (OverlappedComponent :type Primitive%20Component%20Object%20Reference) (OtherActor :type Actor%20Object%20Reference) (OtherComp :type Primitive%20Component%20Object%20Reference) (OtherBodyIndex :type Integer))
  (if (== OtherActor (Variables|Default|GetAs%20BP%20First%20Person%20Character))
    (Utilities|Time|ClearTimerbyFunctionName 0 "DOT")))

(event Custom|DP_Trap_Event
  (params (TrapType :type TrapType%20Enum :default "NewEnumerator0"))
  (if (Utilities|Enum|Equal(Enum) TrapType (Variables|Default|GetTrapType))
    (Collision|SetCollisionEnabled (Variables|Default|GetDamageColl) "NoCollision")
    (Components|DestroyComponent (Variables|Default|GetGas))))

(event Custom|DOT
  (Default|DamageUpdate (Variables|Default|GetAs%20BP%20First%20Person%20Character) (Variables|Default|GetGas_Damage)))

(event EventBeginPlay
  (bind _asbp_player (Utilities|Casting|CastToBP_Player (Game|GetPlayerCharacter 0)))
  (bind _output_get (Variables|Default|SetAs%20BP%20First%20Person%20Character _asbp_player))
  (EventDispatchers|BindEventtoDPTrap _output_get (delegate Custom|DP_Trap_Event)))

(fn ConstructionScript)