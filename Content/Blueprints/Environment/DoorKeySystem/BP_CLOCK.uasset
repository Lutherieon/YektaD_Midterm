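; BP_CLOCK is a rotating clock hazard in the DoorKeySystem folder that hurts the player.
; When BP_Player overlaps its Box, a timeline plays, pitching the Scene component by the track value scaled to degrees.
; Every timeline update also damages that player, so damage depends on frame rate and continues without an end-overlap check.
; The construction script sets the Gondol5 material from DoorIndex.
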(event OnComponentBeginOverlap(Box)
  (params (OverlappedComponent :type Primitive%20Component%20Object%20Reference) (OtherActor :type Actor%20Object%20Reference) (OtherComp :type Primitive%20Component%20Object%20Reference) (OtherBodyIndex :type Integer) (bFromSweep :type Boolean) (SweepResult :type Hit%20Result%20Structure%20%28by%20ref%29))
  (bind _asbp_player (Utilities|Casting|CastToBP_Player OtherActor))
  (bind _clocktrack (Timeline|ClockTimeline Play)
    (:Update
      (Default|DamageUpdate _asbp_player 5.0)
      (Transformation|SetRelativeRotation (Variables|Default|GetScene) (Math|Rotator|MakeRotator 0.0 (* _clocktrack 3.6e+02) 0.0) false false))))

(fn ConstructionScript
  (Rendering|Material|SetMaterial (Variables|Default|GetGondol_5) 0 (Utilities|Select :Index (Variables|Default|GetDoorIndex) :Option%200 "/Game/FirstPerson/FPWeapon/Materials/FirstPersonProjectileMaterial.FirstPersonProjectileMaterial" :Option%201 "/Game/StarterContent/Materials/M_CobbleStone_Pebble.M_CobbleStone_Pebble" :Option%202 "/Game/FirstPerson/FPWeapon/Materials/M_FPGun.M_FPGun")))