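; BP_SlidingDoor is a key-locked sliding door, colour-coded green, red or blue by its key index.
; On Interact, it opens only if the first-person game mode's Keys value equals KeyIndex, otherwise printing a message.
; A timeline lerps the door mesh's relative location from StartLocation to FinishRotation, which holds a position despite its name.
; The construction script sizes mesh and collision from GridSize and picks the material.
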(event EventBeginPlay
  (bind _asbp_first_person_game_mode (Utilities|Casting|CastToBP_FirstPersonGameMode (Game|GetGameMode)))
  (Variables|Default|SetAs%20BP%20First%20Person%20Game%20Mode _asbp_first_person_game_mode))

(event EventInteract
  (params (CharRef :type BP%20Player%20Object%20Reference))
  (if (== (Variables|/Game/Blueprints/Player/BP_FirstPersonGameMode.BP_FirstPersonGameMode_C|GetKeys (Variables|Default|GetAs%20BP%20First%20Person%20Game%20Mode)) (Variables|Default|GetKeyIndex))
    (bind _slidetrack (Timeline|DoorSlideTimeline Play)
      (:Update
        (Transformation|SetRelativeLocation (Variables|Default|GetSM_Door) (Math|Vector|Lerp(Vector) (Variables|Default|GetStartLocation) (Variables|Default|GetFinishRotation) _slidetrack) false false)))
    (else
      (Development|PrintString "You Dont Have Correct Key"))))

(fn ConstructionScript
  (bind _gridsize (Variables|Default|GetGridSize))
  (Variables|Default|SetWallLength _gridsize)
  (Variables|Default|SetWallThickness (* _gridsize 0.1))
  (Transformation|SetRelativeScale3D (Variables|Default|GetSM_Door) (Utilities|NewMacro (Math|Vector|MakeVector (Variables|Default|GetWallLength) (Variables|Default|GetWallLength) (Variables|Default|GetWallThickness))))
  (Rendering|Material|SetMaterial (Variables|Default|GetSM_Door) 0 (Utilities|Select :Index (Variables|Default|GetKeyIndex) :Option%200 "/Game/Materials/M_Green.M_Green" :Option%201 "/Game/Materials/M_Red.M_Red" :Option%202 "/Game/Materials/M_Blue.M_Blue")))