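; BP_Spear is a throwable spear weapon that flies as a projectile from the camera's aim.
; Throw stores the camera transform and direction, snaps the spear just ahead of the camera with a yaw correction and pivot offset, then activates ProjectileMovement at a fixed speed, ignoring the passed ThrowSpeed.
; BeginPlay caches the player; StartSpearRotForward only zeroes SpearROT's play rate.
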(event Custom|Throw
  (params (Camera%20Rotation :type Rotator) (ThrowDirectionVector :type Vector) (CameraLocation :type Vector) (ThrowSpeed :type Float%20%28double-precision%29))
  (bind _projectilemovement (Variables|Default|GetProjectileMovement))
  (Variables|Default|SetCameraStartRotation Camera%20Rotation)
  (Variables|Default|SetThrowDirection ThrowDirectionVector)
  (Variables|Default|SetCameraLocationAtThrow CameraLocation)
  (Variables|Default|SetSpearThrowSpeed 2.5e+03)
  (CallFunction|SnapSpeartoStartPoint (Math|Rotator|MakeRotator (.Roll (Math|Rotator|BreakRotator (Variables|Default|GetCameraStartRotation))) (.Pitch (Math|Rotator|BreakRotator (Variables|Default|GetCameraStartRotation))) (+ (.Yaw (Math|Rotator|BreakRotator (Variables|Default|GetCameraStartRotation))) 9e+01)) (Variables|Default|GetThrowDirection) (Variables|Default|GetCameraLocationAtThrow))
  (Variables|/Script/Engine.MovementComponent|SetVelocity _projectilemovement (* (Variables|Default|GetThrowDirection) (Variables|Default|GetSpearThrowSpeed)))
  (Components|Activation|Activate _projectilemovement false))

(event Custom|StartSpearRotForward
  (Components|Timeline|SetPlayRate (Variables|Default|GetSpearROT) 0.0))

(event EventBeginPlay
  ;[0.15 0.15 0.15 0.5] BeginPlayer - Cast To Main Character
  (bind _asbp_player (Utilities|Casting|CastToBP_Player (Game|GetPlayerCharacter 0)))
  (Variables|Default|SetAs%20BP%20First%20Person%20Character _asbp_player))

(fn ConstructionScript)

(fn SnapSpeartoStartPoint
  (params (StartRotation :type Rotator) (ThrowDrectionVector :type Vector) (CameraLocation :type Vector))
  (Transformation|SetActorLocationAndRotation (- (+ (* ThrowDrectionVector 1e+01) CameraLocation) (Variables|/Script/Engine.SceneComponent|GetRelativeLocation (Variables|Default|GetPivotPoint))) StartRotation))