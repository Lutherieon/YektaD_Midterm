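; Throwable axe weapon that the player launches, lodges in surfaces and recalls to hand.
; Throw drives projectile movement with timeline spin and gravity, line-tracing along velocity to lodge the axe at an angle set by the impact normal.
; Recall wiggles or pulls it free, then curves it back with distance-scaled speed and whole-number spins while sphere-tracing.
; Hitting a dungeon door spawns temporary BP_Damage, triggering one-time auto-recall and camera shake.
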(event Custom|Throw
  (params (CameraRotation :type Rotator) (Throw%20Direction%20Vector :type Vector) (CameraLocation :type Vector) (Throw%20Speed :type Float%20%28double-precision%29))
  (bind _returnvalue (Transformation|GetActorLocation))
  (bind _projectilemovement (Variables|Default|GetProjectileMovement))
  ;[0.15 0.15 0.15 0.5] Throw
  (Variables|Default|SetCameraStartRotation CameraRotation)
  (Variables|Default|SetThrowDirection Throw%20Direction%20Vector)
  (Variables|Default|SetCameraLocationAtThrow CameraLocation)
  (Variables|Default|SetAxeThrowSpeed Throw%20Speed)
  ;[0.15 0.15 0.15 0.5] Snap Axe To Start Point
  (CallFunction|SnaptoStartPoint (Math|Rotator|MakeRotator (+ (Variables|Default|GetAxeSpinAxisOffset) (.Roll (Math|Rotator|BreakRotator (Variables|Default|GetCameraStartRotation)))) (.Pitch (Math|Rotator|BreakRotator (Variables|Default|GetCameraStartRotation))) (.Yaw (Math|Rotator|BreakRotator (Variables|Default|GetCameraStartRotation)))) (Variables|Default|GetThrowDirection) (Variables|Default|GetCameraLocationAtThrow))
  ;[0.15 0.15 0.15 0.5] Launch Axe
  (Variables|/Script/Engine.MovementComponent|SetVelocity _projectilemovement (* (Variables|Default|GetThrowDirection) (Variables|Default|GetAxeThrowSpeed)))
  (Components|Activation|Activate _projectilemovement false)
  (CallFunction|StartAxeRotForward)
  (Variables|Default|SetAxeState "NewEnumerator1")
  (Variables|/Script/Engine.ProjectileMovementComponent|SetProjectileGravityScale (Variables|Default|GetProjectileMovement) 0.0)
  ;[0.15 0.15 0.15 0.5] Trace for Hit along velocity on tick
  (bind _newtrack_0 (Timeline|AxeThrowTraceTimeline PlayFromStart)
    (:Update
      (Variables|/Script/Engine.ProjectileMovementComponent|SetProjectileGravityScale (Variables|Default|GetProjectileMovement) _newtrack_0)
      (bind _outhit (Collision|LineTraceByChannel _returnvalue (+ _returnvalue (* (Math|Vector|Normalize (Transformation|GetVelocity)) (Variables|Default|GetAxeThrowTraceDistance))) "TraceTypeQuery1" false 0 "None" true "(R=1.000000,G=0.000000,B=0.000000,A=1.000000)" "(R=0.000000,G=1.000000,B=0.000000,A=1.000000)" 12.0))
      (if (.bBlockingHit (Collision|BreakHitResult _outhit))
        (Variables|Default|SetImpact%20Location (.ImpactPoint (Collision|BreakHitResult _outhit)))
        (Variables|Default|SetImpactNormal (.Normal (Collision|BreakHitResult _outhit)))
        (Variables|Default|SetBone%20Name (.BoneName (Collision|BreakHitResult _outhit)))
        (Variables|Default|SetSurfaceType (Variables|/Script/PhysicsCore.PhysicalMaterial|GetSurfaceType (.PhysMat (Collision|BreakHitResult _outhit))))
        (bind _asgc_sm_dungeon_door (Utilities|Casting|CastToGC_SM_DungeonDoor (.HitActor (Collision|BreakHitResult _outhit)))
          (:then
            (CallFunction|LodgeAxe)
            (bind _returnvalue_2 (Game|SpawnActorfromClass "/Game/Blueprints/BP_Damage.BP_Damage_C" (Transformation|GetWorldTransform (Variables|/Game/Blueprints/Environment/GC_SM_DungeonDoor.GC_SM_DungeonDoor_C|GetDamage _asgc_sm_dungeon_door)) "AdjustIfPossibleButAlwaysSpawn" "MultiplyWithRoot" 0 0))
            (Utilities|FlowControl|Sequence
              (:then_0
                (Utilities|FlowControl|Delay 3.0)
                (Actor|DestroyActor _returnvalue_2))
              (:then_1
                (Utilities|FlowControl|DoOnce false
                  (:Completed
                    (Default|RecallAxe (Variables|Default|GetAs%20BP%20First%20Person%20Character)))))
              (:then_2
                (Utilities|FlowControl|DoOnce false
                  (:Completed
                    (bind _asplayer_controller (Utilities|Casting|CastToPlayerController (Game|GetPlayerController 0)))
                    (Game|Feedback|ClientStartCameraShake _asplayer_controller "/Game/Blueprints/BP_CameraShake.BP_CameraShake_C" 1.0 "World" "0, 0, 0"))))))
          (:CastFailed
            (Components|Activation|Deactivate (Variables|Default|GetProjectileMovement))
            (CallFunction|LodgeAxe)))))
    (:Finished
      ;[0.15 0.15 0.15 0.5] Time out and stop moving once axe is out of view
      (CallFunction|StopAxeMoving)
      (Rendering|SetVisibility (Variables|Default|GetSkeletalMesh) false false))))

(event Custom|StartAxeRotForward
  ;[0.15 0.15 0.15 0.5] Axe Throw Rotation
  (Components|Timeline|SetPlayRate (Variables|Default|GetAxeRotationTimeline) (Variables|Default|GetAxeSpinRate))
  (bind _rotation (Timeline|AxeRotationTimeline PlayFromStart)
    (:Update
      (Transformation|SetRelativeRotation (Variables|Default|GetPivotPoint) (Math|Rotator|MakeRotator 0.0 (* _rotation -3.6e+02) 0.0) false false))
    (:Auido
      ;;[0.2448 0 0.1882] Audio
      (Utilities|FlowControl|FlipFlop
        (:A
          (Audio|PlaySound2D 0 1.0 1.0 0.0 0 0))
        (:B
          (Audio|PlaySound2D 0 1.0 1.0 0.0 0 0))))))

(event Custom|StopAxeRotation
  ;[0.15 0.15 0.15 0.5] Axe Throw Rotation
  (bind _rotation (Timeline|AxeRotationTimeline Stop)
    (:Update
      (Transformation|SetRelativeRotation (Variables|Default|GetPivotPoint) (Math|Rotator|MakeRotator 0.0 (* _rotation -3.6e+02) 0.0) false false))
    (:Auido
      ;;[0.2448 0 0.1882] Audio
      (Utilities|FlowControl|FlipFlop
        (:A
          (Audio|PlaySound2D 0 1.0 1.0 0.0 0 0))
        (:B
          (Audio|PlaySound2D 0 1.0 1.0 0.0 0 0))))))

(event Custom|StopAxeThrowTraceTimeline
  (bind _returnvalue (Transformation|GetActorLocation))
  ;[0.15 0.15 0.15 0.5] Trace for Hit along velocity on tick
  (bind _newtrack_0 (Timeline|AxeThrowTraceTimeline Stop)
    (:Update
      (Variables|/Script/Engine.ProjectileMovementComponent|SetProjectileGravityScale (Variables|Default|GetProjectileMovement) _newtrack_0)
      (bind _outhit (Collision|LineTraceByChannel _returnvalue (+ _returnvalue (* (Math|Vector|Normalize (Transformation|GetVelocity)) (Variables|Default|GetAxeThrowTraceDistance))) "TraceTypeQuery1" false 0 "None" true "(R=1.000000,G=0.000000,B=0.000000,A=1.000000)" "(R=0.000000,G=1.000000,B=0.000000,A=1.000000)" 12.0))
      (if (.bBlockingHit (Collision|BreakHitResult _outhit))
        (Variables|Default|SetImpact%20Location (.ImpactPoint (Collision|BreakHitResult _outhit)))
        (Variables|Default|SetImpactNormal (.Normal (Collision|BreakHitResult _outhit)))
        (Variables|Default|SetBone%20Name (.BoneName (Collision|BreakHitResult _outhit)))
        (Variables|Default|SetSurfaceType (Variables|/Script/PhysicsCore.PhysicalMaterial|GetSurfaceType (.PhysMat (Collision|BreakHitResult _outhit))))
        (bind _asgc_sm_dungeon_door (Utilities|Casting|CastToGC_SM_DungeonDoor (.HitActor (Collision|BreakHitResult _outhit)))
          (:then
            (CallFunction|LodgeAxe)
            (bind _returnvalue_2 (Game|SpawnActorfromClass "/Game/Blueprints/BP_Damage.BP_Damage_C" (Transformation|GetWorldTransform (Variables|/Game/Blueprints/Environment/GC_SM_DungeonDoor.GC_SM_DungeonDoor_C|GetDamage _asgc_sm_dungeon_door)) "AdjustIfPossibleButAlwaysSpawn" "MultiplyWithRoot" 0 0))
            (Utilities|FlowControl|Sequence
              (:then_0
                (Utilities|FlowControl|Delay 3.0)
                (Actor|DestroyActor _returnvalue_2))
              (:then_1
                (Utilities|FlowControl|DoOnce false
                  (:Completed
                    (Default|RecallAxe (Variables|Default|GetAs%20BP%20First%20Person%20Character)))))
              (:then_2
                (Utilities|FlowControl|DoOnce false
                  (:Completed
                    (bind _asplayer_controller (Utilities|Casting|CastToPlayerController (Game|GetPlayerController 0)))
                    (Game|Feedback|ClientStartCameraShake _asplayer_controller "/Game/Blueprints/BP_CameraShake.BP_CameraShake_C" 1.0 "World" "0, 0, 0"))))))
          (:CastFailed
            (Components|Activation|Deactivate (Variables|Default|GetProjectileMovement))
            (CallFunction|LodgeAxe)))))
    (:Finished
      ;[0.15 0.15 0.15 0.5] Time out and stop moving once axe is out of view
      (CallFunction|StopAxeMoving)
      (Rendering|SetVisibility (Variables|Default|GetSkeletalMesh) false false))))

(event Custom|Recall
  (bind _axereturnspeed (Variables|Default|GetAxeReturnSpeed))
  (bind _optimaldistance (Variables|Default|GetOptimalDistance))
  (bind _returnvalue (CallFunction|CalculateReturnTimelineSpeed _optimaldistance _axereturnspeed))
  ;[0.15 0.15 0.15 0.5] Stop throw trace and set visible if axe reached end of range
  (CallFunction|StopAxeThrowTraceTimeline)
  (Rendering|SetVisibility (Variables|Default|GetSkeletalMesh) true false)
  ;[0.15 0.15 0.15 0.5] Wiggle/pull axe before return
  (switch Utilities|FlowControl|Switch|SwitchonAxeState (Variables|Default|GetAxeState)
    (:NewEnumerator1
      (Variables|Default|SetZ%20Adjustment 1e+01))
    (:NewEnumerator2
      (if (Variables|Default|GetWiggle/Pull)
        (|AxeLodgeWiggle
          (:Finished
            _))
        (else
          (|AxeLodgePull)))))
  (Variables|Default|SetAxeState "NewEnumerator3")
  (Utilities|FlowControl|Sequence
    (:then_0
      ;[0.15 0.15 0.15 0.5] Initialise return variables
      (Variables|Default|SetDistanceFromChar (CallFunction|GetClampedAxeDistancefromChar (Variables|Default|GetMaxCalculationDistance)))
      (CallFunction|AdjustAxeReturnLocation)
      (Variables|Default|SetInitialLoc (Transformation|GetActorLocation))
      (Variables|Default|SetInitialRot (Transformation|GetActorRotation))
      (Variables|Default|SetCameraStartRotation (Transformation|GetWorldRotation (Variables|/Game/Blueprints/Player/BP_Player.BP_Player_C|GetFirstPersonCamera (Variables|Default|GetAs%20BP%20First%20Person%20Character))))
      (Transformation|SetRelativeRotation (Variables|Default|GetLodgePoint) "0, 0, 0" false false)
      (Components|Timeline|SetPlayRate (Variables|Default|GetAxeReturnCurveTimeline) _returnvalue)
      (Utilities|FlowControl|Sequence
        (:then_0
          (|ReturnPostionAndReturnAudio
            (:Finished
              (Utilities|FlowControl|Sequence
                (:then_0
                  ;[0.15 0.15 0.15 0.5] Axe Return Trace
                  (Timeline|AxeTrace_Return Stop
                    (:Update
                      (bind _outhit (Collision|SphereTraceByChannel (Variables|Default|GetReturnTargetLocation) (Variables|Default|GetAxeLocationLastTick) 25.0 "TraceTypeQuery1" false 0 "None"))
                      (Variables|Default|SetAxeLocationLastTick (Variables|Default|GetReturnTargetLocation))
                      (if (.bBlockingHit (Collision|BreakHitResult _outhit))
                        (Variables|Default|SetImpact%20Location (.ImpactPoint (Collision|BreakHitResult _outhit)))
                        (bind _asgc_sm_dungeon_door (Utilities|Casting|CastToGC_SM_DungeonDoor (.HitActor (Collision|BreakHitResult _outhit)))
                          (:then
                            (CallFunction|LodgeAxe)
                            (bind _returnvalue_2 (Game|SpawnActorfromClass "/Game/Blueprints/BP_Damage.BP_Damage_C" (Transformation|GetWorldTransform (Variables|/Game/Blueprints/Environment/GC_SM_DungeonDoor.GC_SM_DungeonDoor_C|GetDamage _asgc_sm_dungeon_door)) "AdjustIfPossibleButAlwaysSpawn" "MultiplyWithRoot" 0 0))
                            (Utilities|FlowControl|Sequence
                              (:then_0
                                (Utilities|FlowControl|Delay 3.0)
                                (Actor|DestroyActor _returnvalue_2))
                              (:then_1
                                (Utilities|FlowControl|DoOnce false
                                  (:Completed
                                    (Default|RecallAxe (Variables|Default|GetAs%20BP%20First%20Person%20Character)))))
                              (:then_2
                                (Utilities|FlowControl|DoOnce false
                                  (:Completed
                                    (bind _asplayer_controller (Utilities|Casting|CastToPlayerController (Game|GetPlayerController 0)))
                                    (Game|Feedback|ClientStartCameraShake _asplayer_controller "/Game/Blueprints/BP_CameraShake.BP_CameraShake_C" 1.0 "World" "0, 0, 0"))))))
                          (:CastFailed
                            (Components|Activation|Deactivate (Variables|Default|GetProjectileMovement))
                            (CallFunction|LodgeAxe)))))))
                (:then_1
                  (CallFunction|StopAxeMoving)
                  (Default|Catch (Variables|Default|GetAs%20BP%20First%20Person%20Character)))))))
        (:then_1
          (|ReturnSpinAndReturnAudio _returnvalue))))
    (:then_1
      (Variables|Default|SetAxeLocationLastTick (Variables|Default|GetReturnTargetLocation))
      (Timeline|AxeTrace_Return PlayFromStart))))

(event EventBeginPlay
  ;[0.15 0.15 0.15 0.5] Begin Play - Cast to main Character
  (|CallParentFunction)
  (bind _asbp_player (Utilities|Casting|CastToBP_Player (Game|GetPlayerCharacter 0)))
  (Variables|Default|SetAs%20BP%20First%20Person%20Character _asbp_player))

(fn ConstructionScript
  (|CallParentFunction))

(fn SnaptoStartPoint
  (params (StartRotation :type Rotator) (ThrowDirectionVector :type Vector) (CameraLocation :type Vector))
  ;[0.15 0.15 0.15 0.5] SnapToStartPoint
  (Transformation|SetActorLocationAndRotation (- (+ CameraLocation (* ThrowDirectionVector 1e+02)) (Variables|/Script/Engine.SceneComponent|GetRelativeLocation (Variables|Default|GetPivotPoint))) StartRotation))

(fn StopAxeMoving
  ;[0.15 0.15 0.15 0.5] Comment
  (Components|Activation|Deactivate (Variables|Default|GetProjectileMovement))
  (CallFunction|StopAxeRotation))

(fn LodgeAxe
  (CallFunction|StopAxeMoving)
  (Transformation|SetRelativeRotation (Variables|Default|GetPivotPoint) "0, 0, 0" false false)
  (Transformation|SetActorRotation (Variables|Default|GetCameraStartRotation))
  (Transformation|SetRelativeRotation (Variables|Default|GetLodgePoint) (Math|Rotator|MakeRotator (Math|Random|RandomFloatinRange -3.0 -8.0) (CallFunction|AdjustAxeImpactPitch (Variables|Default|GetImpactNormal) (Math|Random|RandomFloatinRange 3e+01 -55.0) (Math|Random|RandomFloatinRange -5.0 -25.0)) 0.0) false false)
  (Transformation|SetActorLocation (CallFunction|AdjustImpactLocation (Variables|Default|GetImpactNormal) (Variables|Default|GetImpact%20Location)) false false)
  (Variables|Default|SetAxeState "NewEnumerator2"))

(fn AdjustAxeImpactPitch
  (params (ImpactNormal :type Vector) (InclinedSurfaceRange :type Float%20%28double-precision%29) (RegularSurfaceRange :type Float%20%28double-precision%29))
  (bind _returnvalue (Math|Rotator|MakeRotationfromAxes ImpactNormal "0, 0, 0" "0, 0, 0"))
  (return (- (select (> (.pitch _returnvalue) 0.0) RegularSurfaceRange InclinedSurfaceRange) (.pitch _returnvalue))))

(fn AdjustImpactLocation
  (params (ImpactNormal :type Vector) (ImpactLocation :type Vector))
  (bind _returnvalue (Math|Rotator|MakeRotationfromAxes ImpactNormal "0, 0, 0" "0, 0, 0"))
  (bind _returnvalue_2 (> (.pitch _returnvalue) 0.0))
  (bind _returnvalue_3 (select _returnvalue_2 (.pitch _returnvalue) 0.0))
  (bind _returnvalue_4 (- _returnvalue_3 9e+01))
  (bind _returnvalue_5 (/ _returnvalue_4 9e+01))
  (bind _returnvalue_6 (* _returnvalue_5 1e+01))
  (Variables|Default|SetZ%20Adjustment _returnvalue_6)
  (return (+ (+ ImpactLocation (Math|Vector|MakeVector 0.0 0.0 _returnvalue_6)) (- (Transformation|GetActorLocation) (Transformation|GetWorldLocation (Variables|Default|GetLodgePoint))))))

(fn GetClampedAxeDistancefromChar
  (params (MaxDistance :type Float%20%28double-precision%29))
  (return (Math|Float|Clamp(Float) (Math|Vector|VectorLength (- (Transformation|GetActorLocation) (Transformation|GetWorldLocation (Variables|/Game/Blueprints/Player/BP_Player.BP_Player_C|GetFirstPersonMesh (Variables|Default|GetAs%20BP%20First%20Person%20Character))))) 0.0 MaxDistance)))

(fn AdjustAxeReturnLocation
  (Transformation|SetActorLocation (+ (Transformation|GetActorLocation) (Math|Vector|MakeVector 0.0 0.0 (+ (* (- 1.0 (/ (Variables|Default|GetZ%20Adjustment) 1e+01)) 3e+01) 2e+01))) false false))

(fn CalculateReturnTimelineSpeed
  (params (OptimalDistance :type Float%20%28double-precision%29) (AxeReturnSpeed :type Float%20%28double-precision%29))
  (return (Math|Float|Clamp(Float) (/ (* OptimalDistance AxeReturnSpeed) (Variables|Default|GetDistanceFromChar)) 0.4 7.0)))