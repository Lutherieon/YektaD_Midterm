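; BP_Switch is an interactable, single-use switch for turning off traps of its configured TrapType: Spike, Axe or Gas.
; The construction script sets its mesh and scale by type, and BeginPlay writes the type name on a text render.
; On Interact it passes the type to CallDPTrap on the BP_Player cached at BeginPlay, prints a debug message and destroys itself.
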(event EventBeginPlay
  (bind _asbp_player (Utilities|Casting|CastToBP_Player (Game|GetPlayerCharacter 0)))
  (Variables|Default|SetAs%20BP%20First%20Person%20Character _asbp_player)
  (Rendering|Components|TextRender|SetText (Variables|Default|GetTextRender) (Utilities|Text|ToText(String) (Utilities|String|EnumtoString (Variables|Default|GetTrapType)))))

(event EventInteract
  (params (CharRef :type BP%20Player%20Object%20Reference))
  (Default|CallDPTrap (Variables|Default|GetAs%20BP%20First%20Person%20Character) (Variables|Default|GetTrapType))
  (Development|PrintString "Turn Of Trap")
  (Actor|DestroyActor))

(fn ConstructionScript
  (switch Utilities|FlowControl|Switch|SwitchonTrapType (Variables|Default|GetTrapType)
    (:NewEnumerator1
      (Components|StaticMesh|SetStaticMesh (Variables|Default|GetStaticMesh) "/Game/Meshes/SM_SpikeTrapMesh.SM_SpikeTrapMesh")
      (Transformation|SetWorldScale3D (Variables|Default|GetStaticMesh) "0.300000,0.300000,0.300000"))
    (:NewEnumerator2
      (Components|StaticMesh|SetStaticMesh (Variables|Default|GetStaticMesh) "/Game/Meshes/SM_Axe.SM_Axe")
      (Transformation|SetWorldScale3D (Variables|Default|GetStaticMesh) "3.000000,3.000000,3.000000"))
    (:NewEnumerator3
      (Components|StaticMesh|SetStaticMesh (Variables|Default|GetStaticMesh) "/Game/LevelPrototyping/Meshes/SM_ChamferCube.SM_ChamferCube")
      (Transformation|SetWorldScale3D (Variables|Default|GetStaticMesh) "0.300000,0.300000,0.300000"))))